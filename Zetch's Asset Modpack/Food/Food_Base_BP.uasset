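; Base Blueprint for an edible food item in a Pavlov modpack that restores health when used.
; On use, it looks up the owning pawn's Pavlov player status and raises health by a fixed amount through the game logic's SetPlayerVitality.
; It then spawns an attenuated eating-crunch sound at the pawn's location and calls Drop to release the consumed item.
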(event Custom|Eat/DestroyItem
  (bind _pawn (Class|PavlovCustomItem|GetOwningPawn))
  (bind _playerstatus (Class|PavlovProxyStatics|GetPavlovPlayerStatusbyPawn _pawn))
  (Class|PavlovGameLogic|SetPlayerVitality (Class|PavlovLibrary|GetGameLogic) (.PlayerState (Utilities|Struct|BreakPavlovPlayerStatus _playerstatus)) (+ (.Health (Utilities|Struct|BreakPavlovPlayerStatus _playerstatus)) 25) -1 -1)
  (CallFunction|PlaySound (Transformation|GetActorLocation (.Pawn (Utilities|Struct|BreakPavlovPlayerStatus _playerstatus))))
  (Class|PavlovCustomItem|Drop true))

(event Custom|Play%20Sound
  (params (NewParam :type Vector))
  (Audio|SpawnSoundatLocation "/Game/CustomMaps/UGC2848649147/Custom_assets/Assets/Food/Human_Eating⧸Crunch_-_Sound_Effect__HD_.Human_Eating⧸Crunch_-_Sound_Effect__HD_" NewParam "0, 0, 0" 2.0 1.0 1.0 "/Game/CustomMaps/UGC2848649147/Custom_assets/Money.Money" 0))

(event EventOnUse
  (CallFunction|Eat/DestroyItem))

(fn ConstructionScript)