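; Pavlov slot machine shop item that charges the interacting player BuyPrice on a server-side interact.
; Three delayed weighted rolls, each re-randomized at every threshold check, set symbol materials on the mesh's reel slots.
; Three matches pay five times the price; the first roll matching either other pays double, but a second-third pair alone pays nothing.
; Wins play a register sound at a hardcoded location and update AmountWon; reels later reset.
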(event OnInteractBoxClient(Pavlov_InteractBox)
  (params (InteractType :type EInteractType%20Enum :default "Grabbed") (HandProxy :type Pavlov%20Hand%20Proxy%20Object%20Reference) (InteractBox :type Pavlov%20Interact%20Box%20Object%20Reference))
  (Class|PavlovHandProxy|ReplicateInteractServer HandProxy InteractType InteractBox))

(event OnInteractBoxServer(Pavlov_InteractBox)
  (params (InteractType :type EInteractType%20Enum :default "Grabbed") (HandProxy :type Pavlov%20Hand%20Proxy%20Object%20Reference) (InteractBox :type Pavlov%20Interact%20Box%20Object%20Reference))
  (CallFunction|Slots HandProxy))

(event Custom|Slots
  (params (Hand%20Proxy :type Pavlov%20Hand%20Proxy%20Object%20Reference))
  (bind _returnvalue (Math|Random|RandomIntegerinRange 0 100))
  (bind _returnvalue_2 (Math|Random|RandomIntegerinRange 0 100))
  (bind _returnvalue_3 (Class|PavlovHandProxy|GetPlayerProxy Hand%20Proxy))
  (bind _returnvalue_4 (Math|Random|RandomIntegerinRange 0 100))
  (bind _returnvalue_5 (Class|PavlovLibrary|GetGameLogic))
  (bind _buy_price (Variables|Default|GetBuy%20Price))
  (bind _staticmesh (Variables|Default|GetStaticMesh))
  (bind _returnvalue_6 (Class|PavlovPlayerProxy|GetPawn _returnvalue_3))
  (bind _returnvalue_7 (* _buy_price 5))
  (bind _returnvalue_8 (* _buy_price 2))
  (bind _playerstate (Variables|/Script/Engine.Pawn|GetPlayerState _returnvalue_6))
  (bind _playerstatus (Class|PavlovProxyStatics|GetPavlovPlayerStatus _playerstate))
  (if (>= (.Cash (Utilities|Struct|BreakPavlovPlayerStatus _playerstatus)) (Variables|Default|GetBuy%20Price))
    (Class|PavlovGameLogic|SetPlayerCash (Class|PavlovLibrary|GetGameLogic) (.PlayerState (Utilities|Struct|BreakPavlovPlayerStatus _playerstatus)) (- (.Cash (Utilities|Struct|BreakPavlovPlayerStatus _playerstatus)) (Variables|Default|GetBuy%20Price)))
    ;[1 1 1] Roll 1
    (if (Math|Integer|InRange(Integer) _returnvalue_2 0 30)
      (Variables|Default|SetRoll%20Result%201 0)
      (elif (Math|Integer|InRange(Integer) _returnvalue_2 31 60)
        (Variables|Default|SetRoll%20Result%201 1)
        (elif (Math|Integer|InRange(Integer) _returnvalue_2 61 85)
          (Variables|Default|SetRoll%20Result%201 2)
          (else
            (if (Math|Integer|InRange(Integer) _returnvalue_2 86 100)
              _
              (else
                _))
            (Variables|Default|SetRoll%20Result%201 3)))))
    (Rendering|Material|SetMaterial (Variables|Default|GetStaticMesh) 1 (Utilities|Select :Index (Variables|Default|GetRoll%20Result%201) :Option%200 "/Game/CustomMaps/UGC2848649147/Custom_assets/Assets/shop_stuff/Money1_Mat.Money1_Mat" :Option%201 "/Game/CustomMaps/UGC2848649147/Custom_assets/Assets/shop_stuff/Money3_Mat.Money3_Mat" :Option%202 "/Game/CustomMaps/UGC2848649147/Custom_assets/Assets/shop_stuff/Money5_Mat.Money5_Mat" :Option%203 "/Game/CustomMaps/UGC2848649147/Custom_assets/Assets/shop_stuff/Money1k_Mat.Money1k_Mat"))
    (Utilities|FlowControl|Delay 0.5)
    ;[1 1 1] Roll 2
    (if (Math|Integer|InRange(Integer) _returnvalue_4 0 25)
      (Variables|Default|SetRoll%20Result%202 0)
      (elif (Math|Integer|InRange(Integer) _returnvalue_4 26 50)
        (Variables|Default|SetRoll%20Result%202 1)
        (elif (Math|Integer|InRange(Integer) _returnvalue_4 51 75)
          (Variables|Default|SetRoll%20Result%202 2)
          (else
            (if (Math|Integer|InRange(Integer) _returnvalue_4 76 100)
              _
              (else
                _))
            (Variables|Default|SetRoll%20Result%202 3)))))
    (Rendering|Material|SetMaterial (Variables|Default|GetStaticMesh) 2 (Utilities|Select :Index (Variables|Default|GetRoll%20Result%202) :Option%200 "/Game/CustomMaps/UGC2848649147/Custom_assets/Assets/shop_stuff/Money1_Mat.Money1_Mat" :Option%201 "/Game/CustomMaps/UGC2848649147/Custom_assets/Assets/shop_stuff/Money3_Mat.Money3_Mat" :Option%202 "/Game/CustomMaps/UGC2848649147/Custom_assets/Assets/shop_stuff/Money5_Mat.Money5_Mat" :Option%203 "/Game/CustomMaps/UGC2848649147/Custom_assets/Assets/shop_stuff/Money1k_Mat.Money1k_Mat"))
    (Utilities|FlowControl|Delay 0.5)
    ;[1 1 1] Roll 3
    (if (Math|Integer|InRange(Integer) _returnvalue 0 30)
      (Variables|Default|SetRoll%20Result%203 0)
      (elif (Math|Integer|InRange(Integer) _returnvalue 31 60)
        (Variables|Default|SetRoll%20Result%203 1)
        (elif (Math|Integer|InRange(Integer) _returnvalue 61 85)
          (Variables|Default|SetRoll%20Result%203 2)
          (else
            (if (Math|Integer|InRange(Integer) _returnvalue 86 100)
              _
              (else
                _))
            (Variables|Default|SetRoll%20Result%203 3)))))
    (Rendering|Material|SetMaterial (Variables|Default|GetStaticMesh) 0 (Utilities|Select :Index (Variables|Default|GetRoll%20Result%203) :Option%200 "/Game/CustomMaps/UGC2848649147/Custom_assets/Assets/shop_stuff/Money1_Mat.Money1_Mat" :Option%201 "/Game/CustomMaps/UGC2848649147/Custom_assets/Assets/shop_stuff/Money3_Mat.Money3_Mat" :Option%202 "/Game/CustomMaps/UGC2848649147/Custom_assets/Assets/shop_stuff/Money5_Mat.Money5_Mat" :Option%203 "/Game/CustomMaps/UGC2848649147/Custom_assets/Assets/shop_stuff/Money1k_Mat.Money1k_Mat"))
    ;[1 1 1] Result
    (if (== (Variables|Default|GetRoll%20Result%201) (Variables|Default|GetRoll%20Result%202))
      (if (== (Variables|Default|GetRoll%20Result%202) (Variables|Default|GetRoll%20Result%203))
        (Variables|Default|SetWinning%20Amount _returnvalue_7)
        (Class|PavlovGameLogic|GivePlayerCash _returnvalue_5 _playerstate _returnvalue_7)
        (Audio|SpawnSoundatLocation "/Game/CustomMaps/UGC2848649147/Custom_assets/Cash_Register__Kaching__-_Sound_Effect__HD_.Cash_Register__Kaching__-_Sound_Effect__HD_" "180524.312500,-5193.020508,7929.575195" "0, 0, 0" 2.0 1.0 0.0 "/Game/CustomMaps/UGC2848649147/Custom_assets/Money.Money" 0 :!label _label)
        (Rendering|Components|TextRender|SetText (Variables|Default|GetAmount%20Won) (Utilities|Text|ToText(String) (Utilities|String|Append "$" (Utilities|String|ToString(Integer) (Variables|Default|GetWinning%20Amount)))))
        (Variables|Default|SetWinning%20Amount 0)
        (else
          (if (== (Variables|Default|GetRoll%20Result%203) (Variables|Default|GetRoll%20Result%201)) :!label _label_2
            (Variables|Default|SetWinning%20Amount _returnvalue_8 :!label _label_3)
            (Class|PavlovGameLogic|GivePlayerCash _returnvalue_5 _playerstate _returnvalue_8)
            (goto _label)
            (elif (== (Variables|Default|GetRoll%20Result%201) (Variables|Default|GetRoll%20Result%202))
              (goto _label_3)
              (else
                _)))))
      (else
        (goto _label_2)))
    (Utilities|FlowControl|Delay 2.0)
    (Rendering|Material|SetMaterial _staticmesh 1 "/Game/CustomMaps/UGC2848649147/ModularBuildingSet/materials/Decals_Signs/x_alpha_dark.x_alpha_dark")
    (Rendering|Material|SetMaterial _staticmesh 2 "/Game/CustomMaps/UGC2848649147/ModularBuildingSet/materials/Decals_Signs/x_alpha_dark.x_alpha_dark")
    (Rendering|Material|SetMaterial _staticmesh 0 "/Game/CustomMaps/UGC2848649147/ModularBuildingSet/materials/Decals_Signs/x_alpha_dark.x_alpha_dark")))

(fn ConstructionScript)